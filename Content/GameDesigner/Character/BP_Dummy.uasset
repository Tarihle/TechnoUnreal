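; BP_Dummy is a training dummy that plays a pushed animation when damaged and can act as a periodic noise source.
; On BeginPlay, a non-negative SoundInterval starts a looping timer that plays a sound at the dummy's location and reports an AI noise event limited to SoundRange.
; The construction script flushes persistent debug lines, then draws a horizontal debug circle showing that range when it is positive.
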(event Custom|PlaySound
  (bind _self self)
  (bind _returnvalue (Transformation|GetActorLocation _self))
  (Audio|PlaySoundatLocation (Variables|Dummy|GetSound) _returnvalue "0, 0, 0" 1.0 1.0 0.0 0 0 0 0)
  (Class|AISenseHearing|ReportNoiseEvent _returnvalue 1.0 self (Variables|Dummy|GetSoundRange) "None"))

(event Game|Damage|EventAnyDamage
  (params (Damage :type Float%20%28single-precision%29) (DamageType :type Damage%20Type%20Object%20Reference) (InstigatedBy :type Controller%20Object%20Reference) (DamageCauser :type Actor%20Object%20Reference))
  (Components|Animation|PlayAnimation (Variables|Character|GetMesh) "/Game/GameDesigner/Character/Mesh/training_dummy_Anim_ARM_training_dummy_pushed.training_dummy_Anim_ARM_training_dummy_pushed" false))

(event EventBeginPlay
  (bind _soundinterval (Variables|Dummy|GetSoundInterval))
  (if (not (< _soundinterval 0.0))
    (Utilities|Time|SetTimerbyEvent (delegate Custom|PlaySound) _soundinterval true)))

(fn ConstructionScript
  (Rendering|Debug|FlushPersistentDebugLines)
  (if (> (Variables|Dummy|GetSoundRange) 0.0)
    (Rendering|Debug|DrawDebugCircle (Transformation|GetActorLocation self) (Variables|Dummy|GetSoundRange) 12 "(R=0.603029,G=0.000000,B=1.000000,A=1.000000)" 999.0 2.0 "1.000000,0.000000,0.000000" "0.000000,1.000000,0.000000")))