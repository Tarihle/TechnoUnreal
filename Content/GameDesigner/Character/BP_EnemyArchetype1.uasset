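; Enemy character archetype with crouch handling and helpers for firing projectiles at a target actor.
; Crouch events shift every skeletal mesh body part vertically by twice the half-height adjustment, using a component array lazily cached by reference.
; SpawnBullet launches a first-person projectile from a right-hand socket, rotated toward the target.
; A separate helper computes arced launch velocity, which SpawnBullet does not use.
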(event EventOnStartCrouch
  (params (HalfHeightAdjust :type Float%20%28single-precision%29) (ScaledHalfHeightAdjust :type Float%20%28single-precision%29))
  (for _array_element (CallFunction|CacheAllPartsOnce (Variables|Default|GetBodyParts))
    (Transformation|AddRelativeLocation _array_element (Math|Vector|MakeVector 0.0 0.0 (* HalfHeightAdjust 2.0)) false false)))

(event EventOnEndCrouch
  (params (HalfHeightAdjust :type Float%20%28single-precision%29) (ScaledHalfHeightAdjust :type Float%20%28single-precision%29))
  (for _array_element (CallFunction|CacheAllPartsOnce (Variables|Default|GetBodyParts))
    (Transformation|AddRelativeLocation _array_element (Math|Vector|MakeVector 0.0 0.0 (* HalfHeightAdjust -2.0)) false false)))

(fn ConstructionScript)

(fn SpawnBullet
  (params (Actor :type Actor%20Object%20Reference))
  (bind _sc_testconnector (Variables|Default|GetSC_TestConnector))
  (bind _returnvalue (Transformation|GetSocketLocation _sc_testconnector "pinky_metacarpal_r"))
  (Game|SpawnActorfromClass "/Game/FirstPerson/Blueprints/BP_FirstPersonProjectile.BP_FirstPersonProjectile_C" (Math|Transform|MakeTransform _returnvalue (Math|Rotator|FindLookatRotation _returnvalue (Transformation|GetActorLocation Actor)) "1.000000,1.000000,1.000000") "Undefined" "MultiplyWithRoot" 0 0))

(fn GetProjectileTrajectory
  (params (StartPos :type Vector) (EndPos :type Vector) (OverrideGravityZ :type Float%20%28single-precision%29) (ArcParam :type Float%20%28single-precision%29))
  (bind _outlaunchvelocity (Game|SuggestProjectileVelocityCustomArc StartPos EndPos OverrideGravityZ ArcParam))
  (return _outlaunchvelocity))

(fn CacheAllPartsOnce
  (params (RefArray :type Array%20of%20Skeletal%20Mesh%20Component%20Object%20References))
  (if (Utilities|Array|IsNotEmpty RefArray)
    _
    (else
      (|SetBy-RefVar (Actor|GetComponentsByClass "/Script/Engine.SkeletalMeshComponent") RefArray)))
  (return RefArray))