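; Locomotion body-part component that spins itself in proportion to the owning character's horizontal speed.
; One tick after BeginPlay it clears its leader pose and adds a RotatingMovementComponent to the owner, targeting itself with a raised pivot.
; On each character movement update, the XY length of the old velocity becomes the single-axis rotation rate, so the spin follows speed regardless of travel direction.
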(event Custom|OnMove
  (params (DeltaSeconds :type Float%20%28single-precision%29) (OldLocation :type Vector) (OldVelocity :type Vector))
  (Variables|/Script/Engine.RotatingMovementComponent|SetRotationRate (Variables|Default|GetRotator) (Math|Rotator|MakeRotator 0.0 0.0 (Math|Vector|VectorLengthXY OldVelocity))))

(event EventBeginPlay
  (|CallParentFunction)
  (Utilities|FlowControl|DelayUntilNextTick)
  (Components|SkinnedMesh|SetLeaderPoseComponent 0 true false)
  (bind _returnvalue (Game|AddComponentbyClass (Components|GetOwner) "/Script/Engine.RotatingMovementComponent"))
  (bind _output_get (Variables|Default|SetRotator _returnvalue))
  (Components|Movement|SetUpdatedComponent _returnvalue self)
  (Variables|/Script/Engine.RotatingMovementComponent|SetRotationRate _output_get "0, 0, 0")
  (Variables|/Script/Engine.RotatingMovementComponent|SetPivotTranslation _output_get "0.000000,0.000000,45.000000")
  (bind _ascharacter (Utilities|Casting|CastToCharacter (Components|GetOwner)))
  (Character|BindEventtoOnCharacterMovementUpdated _ascharacter (delegate Custom|OnMove)))

(event EventTick
  (params (DeltaSeconds :type Float%20%28single-precision%29)))