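; SC_LocomotionW1 is a locomotion body-part component, apparently a wheel, meant to spin with its owning character's horizontal speed.
; OnMove sets a RotatingMovementComponent's single-axis rotation rate from the XY velocity length.
; The setup that creates that rotator around a raised pivot and binds OnMove to the character's movement update is disconnected from the empty BeginPlay, so the spin is inactive as written.
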(event Custom|OnMove
  (params (DeltaSeconds :type Float%20%28single-precision%29) (OldLocation :type Vector) (OldVelocity :type Vector))
  (Variables|/Script/Engine.RotatingMovementComponent|SetRotationRate (Variables|Default|GetRotator) (Math|Rotator|MakeRotator 0.0 0.0 (Math|Vector|VectorLengthXY OldVelocity))))

(event EventBeginPlay)