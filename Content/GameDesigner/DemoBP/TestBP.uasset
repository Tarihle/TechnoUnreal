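; Demo test actor that spawns and clears batches of BP_EnemyArchetype, with an on-screen counter.
; On BeginPlay it enables player input and creates WBP_Counter with a reference to itself.
; T spawns a batch at the actor's transform, sized by Amount, giving each enemy a random skeletal mesh from BodyVariation.
; R destroys all tracked enemies; both keys broadcast the new count through OnAmountChange.
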(event EventBeginPlay
  (bind _returnvalue (UserInterface|CreateWidget "/Game/GameDesigner/DemoBP/WBP_Counter.WBP_Counter_C" 0 self))
  (UserInterface|Viewport|AddtoViewport _returnvalue 0)
  (Input|EnableInput (Game|GetPlayerController 0)))

(event Input|KeyboardEvents|R
  (params (Key :type Key%20Structure :default "None"))
  (bind _placed_actors (Variables|Default|GetPlaced%20Actors))
  (:Pressed
    (for _array_element _placed_actors
      (Actor|DestroyActor _array_element))
    (Utilities|Array|Clear _placed_actors)
    (Default|CallOnAmountChange)))

(event Input|KeyboardEvents|T
  (params (Key :type Key%20Structure :default "None"))
  (:Pressed
    (for _index (range 0 (Variables|Default|GetAmount))
      (bind _returnvalue (Game|SpawnActorfromClass "/Game/GameDesigner/Character/BP_EnemyArchetype.BP_EnemyArchetype_C" (Transformation|GetActorTransform self) "AdjustIfPossibleButAlwaysSpawn" "MultiplyWithRoot" 0 0))
      (Components|SkeletalMesh|SetSkeletalMeshAsset (Variables|/Game/GameDesigner/Character/BP_EnemyArchetype.BP_EnemyArchetype_C|GetSC_TestConnector _returnvalue) (.OutItem (Utilities|Array|Random (Variables|Default|GetBodyVariation))))
      (Utilities|Array|Add (Variables|Default|GetPlaced%20Actors) _returnvalue))
    (Default|CallOnAmountChange (Utilities|Array|Length (Variables|Default|GetPlaced%20Actors)))))

(fn ConstructionScript)