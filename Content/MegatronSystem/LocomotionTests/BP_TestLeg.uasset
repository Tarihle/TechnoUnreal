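; BP_TestLeg is a test Blueprint for the Megatron system's locomotion tests that exercises TestLegTask on a third-person character owner.
; BeginPlay caches the owning character, and an auto-generated-style function executes the task.
; Crouch handlers print whether the task is valid or finish it as successful, and a success handler prints confirmation.
; The bindings for crouch and task-success events sit in unconnected nodes that never run.
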(event Custom|CrouchEvent
  (Utilities|IsValid (Class|BodyPart|GetTask "(TagName=\"MegatronTask.TestLegTask\")")
    (:Is%20Valid
      (Development|PrintString "TASK" true true "(R=0.311280,G=0.275120,B=1.000000,A=1.000000)"))
    (:Is%20Not%20Valid
      (Development|PrintString "INVALID TASK" true true "(R=1.000000,G=0.112673,B=0.000000,A=1.000000)"))))

(event Custom|TaskSuccess
  (Development|PrintString "OnTaskSuccess" true true "(R=0.279981,G=1.000000,B=0.000000,A=1.000000)"))

(event Custom|FinishCrouch
  (bind _returnvalue (Class|BodyPart|GetTask "(TagName=\"MegatronTask.TestLegTask\")"))
  (Utilities|IsValid _returnvalue
    (:Is%20Valid
      (Class|MegatronTask|Finish _returnvalue true))))

(event EventTick
  (params (DeltaSeconds :type Float%20%28single-precision%29)))

(event EventBeginPlay
  (bind _asbp_third_person_character (Utilities|Casting|CastToBP_ThirdPersonCharacter (Components|GetOwner)))
  (bind _output_get (Variables|Default|SetOwnerTPChar _asbp_third_person_character)))

(fn BPTestLegAutoGenFunc
  (Class|MegatronTask|Execute (Class|BodyPart|GetTask "(TagName=\"MegatronTask.TestLegTask\")")))