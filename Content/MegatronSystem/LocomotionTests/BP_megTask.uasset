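; BP_megTask is a task Blueprint in the MegatronSystem locomotion tests that runs for a few ticks and then finishes, logging as it goes.
; Execute calls the parent, resets the iteration counter and prints the task's display name.
; Each Tick increments and prints the counter, then calls Finish with true and prints a green completion message once it reaches five.
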(fn Execute
  (|CallParentFunction)
  (Variables|Default|Setiterations 0)
  (Development|PrintString 0 (Utilities|String|Append (Utilities|GetDisplayName self) ": Execute") true true "(R=0.049087,G=0.000000,B=1.000000,A=1.000000)" 3.0)
  (return))

(fn Tick
  (params (DeltaSeconds :type Float%20%28single-precision%29))
  (bind _result (Math|Integer|IncrementInt (Variables|Default|Getiterations))
    (:%20%20
      (Development|PrintString 0 (Utilities|String|Append "tick number " (Utilities|String|ToString(Integer) _result)))
      (if (>= _result 5)
        (Class|MegatronTask|Finish true)
        (Development|PrintString 0 "finished task" true true "(R=0.351638,G=1.000000,B=0.000000,A=1.000000)")))))